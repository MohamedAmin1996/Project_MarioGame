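; BP_MyEnemy is a platformer-style enemy that moves on its own and is killed when the player jumps on it.
; Each tick it calls MoveEnemy, noted as a C++ variant, passing speed, distance, fall-avoidance and front/fall trace settings.
; On box overlap with a Player-tagged actor, a height comparison decides whether the player bounces up and the enemy is destroyed, or the LoseMap level opens.
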(event `self.ReceiveActorBeginOverlap`
  (params (OtherActor :type "Actor Object Reference")))

(event `self.ReceiveTick`
  (params (DeltaSeconds :type "Float (single-precision)"))
  ;[1 1 1] MoveEnemy() - C++ variant
  (`self.MoveEnemy` (`self.WillNotFall`) DeltaSeconds (`self.Speed`) (`self.LocationDistance`) (`self.LineTraceFallDistance`) (`self.LineTraceFrontDistance`)))

(event `self.BoxCollider.OnComponentBeginOverlap`
  (params (OverlappedComponent :type "PrimitiveComponent Object Reference") (OtherActor :type "Actor Object Reference") (OtherComp :type "PrimitiveComponent Object Reference") (OtherBodyIndex :type Integer) (bFromSweep :type Boolean) (SweepResult :type "HitResult Structure (by ref)"))
  (bind (_returnvalue_x _returnvalue_y _returnvalue_z) (`KismetMathLibrary.BreakVector` (`self.K2_GetActorLocation`)))
  (bind (_returnvalue_x_2 _returnvalue_y_2 _returnvalue_z_2) (`KismetMathLibrary.BreakVector` (`self.K2_GetActorLocation` OtherActor)))
  ;[1 1 1] Checking if player jump on this actor or has collided from the sides
  (if (`self.ActorHasTag` OtherActor "Player")
    (if (> _returnvalue_z_2 (+ _returnvalue_z 10.0))
      (`PrimitiveComponent.AddImpulse` OtherComp (0.0 0.0 1000.0) "None" false)
      (`self.K2_DestroyActor`)
      (else
        (`GameplayStatics.OpenLevel` "LoseMap")))))

(fn `UserConstructionScript`)