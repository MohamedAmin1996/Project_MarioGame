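; Player Blueprint for a character that moves along a left/right axis and jumps, built on a cube component.
; The MoveRight axis flips the actor's yaw at full input and feeds MovePlayer, commented as a C++ variant, with a Blueprint movement version left disconnected.
; Jump applies an upward impulse to the cube unless airborne.
; Any actor overlap clears the airborne flag, as the Ground tag check is unused.
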(event `InputAction|JumpButton`
  (params (Key :type "Key Structure"))
  ;[1 1 1] Jump() - Blueprint function variant
  (:`Pressed`
    (`self.Jump`)))

(event `self.ReceiveActorBeginOverlap`
  (params (OtherActor :type "Actor Object Reference"))
  ;[1 1 1] Jump() - Blueprint function variant
  (set `self.isInTheAir` false))

(event `InputAxis|MoveRight`
  (params (AxisValue :type "Float (single-precision)"))
  (bind (_returnvalue_roll _returnvalue_pitch) (`KismetMathLibrary.BreakRotator` (`self.K2_GetActorRotation`)))
  (bind (_returnvalue_roll_2 _returnvalue_pitch_2) (`KismetMathLibrary.BreakRotator` (`self.K2_GetActorRotation`)))
  ;[1 1 1] Rotate actor based of input direction
  (if (== AxisValue 1.0)
    (`self.K2_SetActorRotation` (`KismetMathLibrary.MakeRotator` 0.0 _returnvalue_pitch_2))
    (elif (== AxisValue -1.0)
      (`self.K2_SetActorRotation` (`KismetMathLibrary.MakeRotator` 0.0 _returnvalue_pitch 180.0)))))

(event `InputAxis|MoveRight`
  (params (AxisValue :type "Float (single-precision)"))
  ;[1 1 1] MovePlayer() - C++ variant
  (`self.MovePlayer` (`GameplayStatics.GetWorldDeltaSeconds`) (`self.Speed`) AxisValue))

(fn `Jump`
  (if (not (`self.isInTheAir`))
    (`PrimitiveComponent.AddImpulse` (`self.Cube`) (`KismetMathLibrary.MakeVector` 0.0 0.0 (`self.JumpHeight`)) "None" false)
    (set `self.isInTheAir` true)))

(fn `UserConstructionScript`)